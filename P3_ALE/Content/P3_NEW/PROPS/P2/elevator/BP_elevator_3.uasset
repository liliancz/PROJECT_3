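; BP_elevator_3 is an elevator prop with two sliding doors that the player opens by pressing O.
; Its Box overlap enables input while FirstPersonCharacter is inside and disables it on exit.
; O plays a timeline that lerps LEFT and RIGHT between stored start and end relative locations, then a delay reverses it to close them after five seconds.
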(event OnComponentBeginOverlap(Box)
  (params (OverlappedComponent :type Primitive%20Component%20Object%20Reference) (OtherActor :type Actor%20Object%20Reference) (OtherComp :type Primitive%20Component%20Object%20Reference) (OtherBodyIndex :type Integer) (bFromSweep :type Boolean) (SweepResult :type Hit%20Result%20Structure%20%28by%20ref%29))
  (Utilities|Casting|CastToFirstPersonCharacter OtherActor)
  (Input|EnableInput (Game|GetPlayerController 0)))

(event OnComponentEndOverlap(Box)
  (params (OverlappedComponent :type Primitive%20Component%20Object%20Reference) (OtherActor :type Actor%20Object%20Reference) (OtherComp :type Primitive%20Component%20Object%20Reference) (OtherBodyIndex :type Integer))
  (Utilities|Casting|CastToFirstPersonCharacter OtherActor)
  (Input|DisableInput (Game|GetPlayerController 0)))

(event EventBeginPlay)

(event Collision|EventActorBeginOverlap
  (params (OtherActor :type Actor%20Object%20Reference)))

(event EventTick
  (params (DeltaSeconds :type Float%20%28single-precision%29)))

(event Input|KeyboardEvents|O
  (params (Key :type Key%20Structure))
  (:Pressed
    (Utilities|FlowControl|Sequence
      (:then_0
        (bind _newtrack_0 (Timeline|Timeline_1 Play)
          (:Update
            (Utilities|FlowControl|Sequence
              (:then_0
                (Transformation|SetRelativeLocation (Variables|Default|GetLEFT) (Math|Vector|Lerp(Vector) (Variables|Default|GetsTART%20POINT) (Variables|Default|GetEnd%20point) _newtrack_0) false false))
              (:then_1
                (Transformation|SetRelativeLocation (Variables|Default|GetRIGHT) (Math|Vector|Lerp(Vector) (Variables|Default|GetsTART%20POINT%201) (Variables|Default|GeteND%20POINT%202) _newtrack_0) false false)))
            (Utilities|FlowControl|Delay 5.0))))
      (:then_1
        (Utilities|FlowControl|Delay 5.0)
        (Timeline|Timeline_1 Reverse)))))

(fn ConstructionScript)